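; BP_Cube is an actor that moves vertically within a 300-unit range above its starting height, driven by custom events.
; Rise, Descend, SetToPercent and SetToMax set a clamped or bounded target Z and start movement, while Stop holds the current height.
; Tick eases toward the target with FInterpTo, then snaps and stops when close.
; SetToMin sets the target but clears the moving flag, so it triggers no descent.
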(event `Rise`
  ;[1 1 1] 注释
  (set `self.TargetZ` (`KismetMathLibrary.FClamp` (+ (`self.TargetZ`) (`self.SmallStep`)) (`self.MinZ`) (`self.MaxZ`)))
  (set `self.bIsMoving` true))

(event `SetToPercent`
  (params (` Percent` :type "Float (double-precision)"))
  ;[1 1 1] 注释
  (set `self.TargetZ` (`KismetMathLibrary.Lerp` (`self.MinZ`) (`self.MaxZ`) (/ (`KismetMathLibrary.FClamp` ` Percent` 0.0 100.0) 100.0)))
  (set `self.bIsMoving` true))

(event `Descend`
  ;[1 1 1] 注释
  (set `self.TargetZ` (`KismetMathLibrary.FClamp` (- (`self.TargetZ`) (`self.SmallStep`)) (`self.MinZ`) (`self.MaxZ`)))
  (set `self.bIsMoving` true))

(event `SetToMin`
  ;[1 1 1] 注释
  (set `self.TargetZ` (`self.MinZ`))
  (set `self.bIsMoving` false))

(event `Stop`
  ;[1 1 1] 注释
  (set `self.TargetZ` (.z (`self.K2_GetActorLocation`)))
  (set `self.bIsMoving` false))

(event `SetToMax`
  ;[1 1 1] 注释
  (set `self.TargetZ` (`self.MaxZ`))
  (set `self.bIsMoving` true))

(event `self.ReceiveTick`
  (params (DeltaSeconds :type "Float (single-precision)"))
  (bind _x (.x (`self.K2_GetActorLocation`)))
  (bind _y (.y (`self.K2_GetActorLocation`)))
  (bind _returnvalue (`KismetMathLibrary.FInterpTo` (.z (`self.K2_GetActorLocation`)) (`self.TargetZ`) DeltaSeconds (`self.InterpSpeed`)))
  ;[1 1 1] 注释
  (if (`self.bIsMoving`)
    (`self.K2_SetActorLocation` (`KismetMathLibrary.MakeVector` _x _y _returnvalue))
    (if (<= (`KismetMathLibrary.Abs` (- _returnvalue (`self.TargetZ`))) 1.0)
      (`self.K2_SetActorLocation` (`KismetMathLibrary.MakeVector` _x _y (`self.TargetZ`)))
      (set `self.bIsMoving` false))))

(event `self.ReceiveBeginPlay`
  ;[1 1 1] 注释
  (bind _output_get (set `self.BaseZ` (.z (`self.K2_GetActorLocation`))))
  (set `self.MinZ` _output_get)
  (set `self.MaxZ` (+ (`self.BaseZ`) 300.0))
  (set `self.TargetZ` (`self.BaseZ`))
  (set `self.bIsMoving` false))

(fn `UserConstructionScript`)